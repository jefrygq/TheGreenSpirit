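; Destructible actor that adds to the game's fear score when it breaks.
; When its Destructible component fractures, it adds FearValue to CausedFear on ThirdPersonGameMode and prints the amount.
; The component hit event is empty, and a duplicate copy of the scoring logic sits unconnected.
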(event OnComponentFracture(Destructible)
  (params (HitPoint :type Vector%20%28by%20ref%29 :default "0, 0, 0") (HitDirection :type Vector%20%28by%20ref%29 :default "0, 0, 0"))
  (bind _fearvalue (Variables|Default|GetFearValue))
  (bind _asthird_person_game_mode (Utilities|Casting|CastToThirdPersonGameMode (Game|GetGameMode)))
  (Variables|/Game/ThirdPersonBP/Blueprints/ThirdPersonGameMode.ThirdPersonGameMode_C|SetCausedFear _asthird_person_game_mode (+ (Variables|/Game/ThirdPersonBP/Blueprints/ThirdPersonGameMode.ThirdPersonGameMode_C|GetCausedFear _asthird_person_game_mode) _fearvalue))
  (Development|PrintString (Utilities|String|ToString(Float) _fearvalue)))

(event OnComponentHit(Destructible)
  (params (HitComponent :type Primitive%20Component%20Object%20Reference) (OtherActor :type Actor%20Object%20Reference) (OtherComp :type Primitive%20Component%20Object%20Reference) (NormalImpulse :type Vector :default "0, 0, 0") (Hit :type Hit%20Result%20Structure%20%28by%20ref%29)))

(event EventBeginPlay)

(event Collision|EventActorBeginOverlap
  (params (OtherActor :type Actor%20Object%20Reference)))

(event EventTick
  (params (DeltaSeconds :type Float%20%28single-precision%29)))

(fn ConstructionScript)