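; Enemy character that carries a sword, takes damage and is destroyed when its HP runs out.
; PawnSensing switches the State enum on sighting any pawn, as the player-controlled check is left unconnected.
; The construction script attaches the sword to the mesh's right-hand socket, and its capsule applies fixed damage to any overlapping actor.
; Incoming damage lowers HP, printing the remainder while the enemy survives.
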(event OnSeePawn(PawnSensing)
  (params (Pawn :type Pawn%20Object%20Reference))
  (Variables|Default|SetState "NewEnumerator1"))

(event OnComponentBeginOverlap(SwordCapsule)
  (params (OverlappedComponent :type Primitive%20Component%20Object%20Reference) (OtherActor :type Actor%20Object%20Reference) (OtherComp :type Primitive%20Component%20Object%20Reference) (OtherBodyIndex :type Integer) (bFromSweep :type Boolean) (SweepResult :type Hit%20Result%20Structure%20%28by%20ref%29))
  (Game|Damage|ApplyDamage OtherActor 2.0 0 0))

(event EventBeginPlay)

(event EventTick
  (params (DeltaSeconds :type Float%20%28single-precision%29)))

(event Game|Damage|EventAnyDamage
  (params (Damage :type Float%20%28single-precision%29) (DamageType :type Damage%20Type%20Object%20Reference) (InstigatedBy :type Controller%20Object%20Reference) (DamageCauser :type Actor%20Object%20Reference))
  (bind _output_get (Variables|Default|SetHP (- (Variables|Default|GetHP) Damage)))
  (if (<= _output_get 0.0)
    (Actor|DestroyActor)
    (else
      (Development|PrintString (Utilities|String|ToString(Float) _output_get)))))

(fn ConstructionScript
  (Transformation|AttachComponentToComponent (Variables|Default|Getsword) (Variables|Character|GetMesh) "hand_r" "KeepRelative" "KeepRelative" "KeepRelative" true))