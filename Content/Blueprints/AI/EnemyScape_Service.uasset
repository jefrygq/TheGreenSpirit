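; Behavior tree service that sets an escape destination for an enemy, based on its position relative to the Morigesh player character.
; Each tick it offsets the pawn's location by its distance to the player and writes the result to the DestinationKey blackboard vector, keeping Z.
; The offset uses cosine of look-at roll for X and sine of pitch for Y, not yaw, so it does not point directly away from the player.
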(event EventReceiveTickAI
  (params (OwnerController :type AI%20Controller%20Object%20Reference) (ControlledPawn :type Pawn%20Object%20Reference) (DeltaSeconds :type Float%20%28single-precision%29))
  (bind _returnvalue (Transformation|GetActorLocation ControlledPawn))
  (bind (_x _y _z) (Math|Vector|BreakVector _returnvalue))
  (bind _asmorigesh_player_character (Utilities|Casting|CastToMorigeshPlayerCharacter (Game|GetPlayerCharacter 0)))
  (AI|BehaviorTree|SetBlackboardValueasVector (Variables|Default|GetDestinationKey) (Math|Vector|MakeVector (+ (* (Math|Trig|Cos(Radians) (.roll (Math|Rotator|FindLookatRotation (Transformation|GetActorLocation _asmorigesh_player_character) _returnvalue))) (Math|Vector|Distance(Vector) (Transformation|GetActorLocation _asmorigesh_player_character) _returnvalue)) _x) (+ (* (Math|Trig|Sin(Radians) (.pitch (Math|Rotator|FindLookatRotation (Transformation|GetActorLocation _asmorigesh_player_character) _returnvalue))) (Math|Vector|Distance(Vector) (Transformation|GetActorLocation _asmorigesh_player_character) _returnvalue)) _y) _z)))